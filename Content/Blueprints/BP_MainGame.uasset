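; Main controller for a grid-based 2D Snake game, spawning the head, food, border walls and HUD on BeginPlay.
; A Delay on Tick paces each step: location comparisons detect collisions, then body parts shift tail-first behind the head.
; Food adds score and a segment and shortens the delay, while arrow keys allow one turn per step.
; Self or wall hits kill the snake and show game over, after which R reloads the level.
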(event Custom|SpawnNewSnakePart
  (params (SpawnLocation :type Vector) (IsHead :type Boolean))
  ;[1 1 1] SpawnNewSnakePart
  (bind _returnvalue (Game|SpawnActorfromClass "/Game/Blueprints/BP_SnakeBodyPart.BP_SnakeBodyPart_C" (Math|Transform|MakeTransform SpawnLocation "0, 0, 0" "1.000000,1.000000,1.000000") "AlwaysSpawn" 0 0))
  (Sprite|SetFlipbook (Variables|/Game/Blueprints/BP_SnakeBodyPart.BP_SnakeBodyPart_C|GetPaperFlipbookBody _returnvalue) (select IsHead "/Game/Flipbooks/RedSquare_Flipbook.RedSquare_Flipbook" "/Game/Flipbooks/YellowSquare_Flipbook.YellowSquare_Flipbook"))
  (Utilities|Array|Add (Variables|Default|GetSnakePartsArray) _returnvalue)
  (Variables|/Game/Blueprints/BP_SnakeBodyPart.BP_SnakeBodyPart_C|SetIsHead _returnvalue IsHead)
  (Transformation|SetActorRotation _returnvalue (Math|Rotator|MakeRotator 0.0 (Utilities|Select :Index (Math|Random|RandomInteger 3) :Option%200 0.0 :Option%201 9e+01 :Option%202 1.8e+02 :Option%203 2.7e+02) 0.0)))

(event Custom|SpawnFood
  (bind _x_max (Variables|Default|GetX_Max))
  (bind _z_max (Variables|Default|GetZ_Max))
  (bind _returnvalue (- _z_max 1e+02))
  (bind _returnvalue_2 (- _x_max 1e+02))
  ;[1 1 1] SpawnFood
  (bind _returnvalue_3 (Game|SpawnActorfromClass "/Game/Blueprints/BP_Food.BP_Food_C" (Math|Transform|MakeTransform (Math|Vector|MakeVector (* (.ReturnValue (Math|Float|Division(WholeandRemainder) (Math|Random|RandomFloatinRange (* _returnvalue_2 -1.0) _returnvalue_2) 1e+02)) 1e+02) -0.1 (* (.ReturnValue (Math|Float|Division(WholeandRemainder) (Math|Random|RandomFloatinRange (* _returnvalue -1.0) _returnvalue) 1e+02)) 1e+02)) "0, 0, 0" "1.000000,1.000000,1.000000") "Undefined" 0 0))
  (Variables|Default|SetFoodActorRef _returnvalue_3))

(event Custom|KillSnake
  ;[1 1 1] KillSnake
  (Variables|Default|SetIsDead true)
  (for (_array_element _array_index) (Variables|Default|GetSnakePartsArray)
    (Sprite|SetFlipbook (Variables|/Game/Blueprints/BP_SnakeBodyPart.BP_SnakeBodyPart_C|GetPaperFlipbookBody _array_element) (select (== _array_index 0) "/Game/Flipbooks/Blank_Flipbook.Blank_Flipbook" "/Game/Flipbooks/Beath_Flipbook.Beath_Flipbook"))
    (Utilities|FlowControl|DoOnce false
      (:Completed
        (Audio|Components|Audio|Stop (Variables|Default|GetMainSound))
        (Audio|PlaySound2D "/Game/Music/Destroy.Destroy" 1.0 1.0 0.0 0 0))))
  (Utilities|FlowControl|Delay 0.5)
  (for _array_element_2 (Variables|Default|GetSnakePartsArray)
    (Sprite|SetFlipbook (Variables|/Game/Blueprints/BP_SnakeBodyPart.BP_SnakeBodyPart_C|GetPaperFlipbookBody _array_element_2) "/Game/Flipbooks/Blank_Flipbook.Blank_Flipbook")))

(event Custom|UpdateScore
  (params (Value :type Integer))
  ;[1 1 1] UpdateScore
  (bind _output_get (Variables|Default|SetScore (+ Value (Variables|Default|GetScore))))
  (Default|UpdateScore (Variables|Default|GetHUD_Ref) _output_get))

(event EventTick
  (params (DeltaSeconds :type Float%20%28single-precision%29))
  (if (Variables|Default|GetIsDead)
    (|RestartSequence)
    (else
      ;[1 1 1] SnakeTick
      (Utilities|FlowControl|Delay (Variables|Default|GetDelay))
      (Utilities|FlowControl|Sequence
        (:then_0
          (|CheckHeadSelfCollision
            (:Completed
              (|CheckWallHeadCollision))))
        (:then_1
          (if (not (Variables|Default|GetIsDead))
            (Utilities|FlowControl|Sequence
              (:then_0
                ;[1 1 1] Food
                (|CheckHeadFoodCollision
                  (:true
                    (|UpdateGameScore)
                    (|DestroyCurrentFood)
                    (|SpawnSnakeNewPart)
                    (CallFunction|SpawnFood)
                    (|SpeedUpSnake))))
              (:then_1
                (|MoveSnake)))))))))

(event EventBeginPlay
  (Input|EnableInput (Game|GetPlayerController 0))
  (bind _returnvalue (Audio|SpawnSound2D "/Game/Music/MainMusic.MainMusic" 1.0 1.0 0.0 0))
  (bind _output_get (Variables|Default|SetMainSound _returnvalue))
  (Audio|Components|Audio|FadeIn _output_get 7.0 1.0 0.0 "Linear" :!class /Script/Engine.AudioComponent)
  (|CreateHudWidget
    (:next
      (|SelectRandomStartDirection
        (:Next
          (Variables|Default|SetDelay (Variables|Default|GetDelay))
          (|SpawnSnakeHead
            (:Next
              (CallFunction|SpawnFood)
              ;[1 1 1] SpawnWall
              (|SpawnWalls))))))))

(event Input|KeyboardEvents|Down
  (params (Key :type Key%20Structure :default "None"))
  ;[1 1 1] Input
  (:Pressed
    (Development|PrintString "Down")
    (if (and (== (Variables|Default|GetDirectionZ) 0) (Variables|Default|GetCanChangeDirection))
      (Variables|Default|SetDirectionX 0)
      (Variables|Default|SetDirectionZ -1)
      (Variables|Default|SetCanChangeDirection false))))

(event Input|KeyboardEvents|Left
  (params (Key :type Key%20Structure :default "None"))
  ;[1 1 1] Input
  (:Pressed
    (Development|PrintString "Left")
    (if (and (== (Variables|Default|GetDirectionX) 0) (Variables|Default|GetCanChangeDirection))
      (Variables|Default|SetDirectionX -1)
      (Variables|Default|SetDirectionZ 0)
      (Variables|Default|SetCanChangeDirection false))))

(event Input|KeyboardEvents|Right
  (params (Key :type Key%20Structure :default "None"))
  ;[1 1 1] Input
  (:Pressed
    (Development|PrintString "Right")
    (if (and (== (Variables|Default|GetDirectionX) 0) (Variables|Default|GetCanChangeDirection))
      (Variables|Default|SetDirectionX 1)
      (Variables|Default|SetDirectionZ 0)
      (Variables|Default|SetCanChangeDirection false))))

(event Input|KeyboardEvents|Up
  (params (Key :type Key%20Structure :default "None"))
  ;[1 1 1] Input
  (:Pressed
    (Development|PrintString "Up")
    (if (and (== (Variables|Default|GetDirectionZ) 0) (Variables|Default|GetCanChangeDirection))
      (Variables|Default|SetDirectionX 0)
      (Variables|Default|SetDirectionZ 1)
      (Variables|Default|SetCanChangeDirection false))))

(event Input|KeyboardEvents|R
  (params (Key :type Key%20Structure :default "None"))
  (:Pressed
    (|RestartSequence) ; enters at Open
  ))

(fn ConstructionScript)

(event Custom|BreakSeflCollisionTestLoop
  (Utilities|Array|ForEachLoopwithBreak (Variables|Default|GetSnakePartsArray)) ; enters at Break
)

(event Custom|BreackWallColTestLoop
  (Utilities|Array|ForEachLoopwithBreak (Variables|Default|GetWallBlocksArray)) ; enters at Break
)

(event Input|KeyboardEvents|Right
  (params (Key :type Key%20Structure))
  (:Pressed
    (Utilities|FlowControl|Gate true) ; enters at Open
  )
  (:Released
    (Utilities|FlowControl|Gate true) ; enters at Close
  ))

(event Input|KeyboardEvents|Left
  (params (Key :type Key%20Structure))
  (:Pressed
    (Utilities|FlowControl|Gate true) ; enters at Open
  )
  (:Released
    (Utilities|FlowControl|Gate true) ; enters at Close
  ))

(event Input|KeyboardEvents|Down
  (params (Key :type Key%20Structure))
  (:Pressed
    (Utilities|FlowControl|Gate true) ; enters at Open
  )
  (:Released
    (Utilities|FlowControl|Gate true) ; enters at Close
  ))

(event Input|KeyboardEvents|Up
  (params (Key :type Key%20Structure))
  (:Pressed
    (Utilities|FlowControl|Gate true) ; enters at Open
  )
  (:Released
    (Utilities|FlowControl|Gate true) ; enters at Close
  ))